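; Test actor that renders a custom shader pass into the RT_SimpleColor render target with a selectable solid color.
; Every Tick it calls DrawTestShaderRenderTarget, passing itself and its Color variable.
; Number keys 1 to 4 switch Color between red, green, blue and magenta, so the next draw picks up the change.
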(event EventBeginPlay)

(event Collision|EventActorBeginOverlap
  (params (OtherActor :type Actor%20Object%20Reference)))

(event EventTick
  (params (DeltaSeconds :type Float%20%28single-precision%29))
  ;[1 1 1] 每帧渲染一次 Custom Pass
  (Class|SimpleColorPassBlueprintLibrary|DrawTestShaderRenderTarget "/Game/RT_SimpleColor.RT_SimpleColor" self (Variables|Default|GetColor)))

(event Input|KeyboardEvents|1
  (params (Key :type Key%20Structure :default "None"))
  ;[1 1 1] 按 数字键改颜色
  (:Pressed
    (Variables|Default|SetColor "(R=1.000000,G=0.000000,B=0.000000,A=1.000000)")))

(event Input|KeyboardEvents|2
  (params (Key :type Key%20Structure :default "None"))
  ;[1 1 1] 按 数字键改颜色
  (:Pressed
    (Variables|Default|SetColor "(R=0.000000,G=1.000000,B=0.000000,A=1.000000)")))

(event Input|KeyboardEvents|3
  (params (Key :type Key%20Structure :default "None"))
  ;[1 1 1] 按 数字键改颜色
  (:Pressed
    (Variables|Default|SetColor "(R=0.000000,G=0.000000,B=1.000000,A=1.000000)")))

(event Input|KeyboardEvents|4
  (params (Key :type Key%20Structure :default "None"))
  ;[1 1 1] 按 数字键改颜色
  (:Pressed
    (Variables|Default|SetColor "(R=0.939640,G=0.000000,B=1.000000,A=1.000000)")))

(fn ConstructionScript)